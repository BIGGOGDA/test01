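; BP_Player is the player pawn, driven by Enhanced Input for movement, rotation and spring-arm zoom.
; BeginPlay adds the Default mapping context through BP_PlayerController.
; Rotation input turns an Arrow with clamped pitch, whose forward and right vectors steer movement at fixed height, unswept and without delta-time scaling.
; Distance input adjusts clamped spring-arm length, and rotation prints a leftover debug string.
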(event `self.ReceiveBeginPlay`
  (bind _asbp_player_controller (cast `/Game/Original/Blueprints/BP_PlayerController` (`self.GetController`)))
  (bind _returnvalue (pcsubsystem `EnhancedInputLocalPlayerSubsystem` _asbp_player_controller))
  (`/Engine/EditorBlueprintResources/StandardMacros.IsValid` _returnvalue
    (:`Is Valid`
      (`EnhancedInputSubsystemInterface.AddMappingContext` _returnvalue "/Game/Original/Input/Default.Default" 0 (struct)))))

(event `EnhancedInput|/Game/Original/Input/InputAsset/Move`
  (params (ActionValue :type "Vector2D Structure") (ElapsedSeconds :type "Float (double-precision)") (TriggeredSeconds :type "Float (double-precision)") (InputAction :type "InputAction Object Reference" :default "/Game/Original/Input/InputAsset/Move.Move"))
  (bind (_x _y) (`KismetMathLibrary.BreakVector2D` ActionValue))
  (bind _returnvalue (`self.K2_GetActorLocation`))
  (bind _arrow (`self.Arrow`))
  (:`Triggered`
    (`self.K2_SetActorLocation` (`KismetMathLibrary.MakeVector` (.x (+ (* (+ (* (`SceneComponent.GetForwardVector` _arrow) _x) (* _y (`SceneComponent.GetRightVector` _arrow))) (`self.MoveSpeed`)) _returnvalue)) (.y (+ (* (+ (* (`SceneComponent.GetForwardVector` _arrow) _x) (* _y (`SceneComponent.GetRightVector` _arrow))) (`self.MoveSpeed`)) _returnvalue)) (.z _returnvalue)))))

(event `EnhancedInput|/Game/Original/Input/InputAsset/Rotation`
  (params (ActionValue :type "Vector2D Structure") (ElapsedSeconds :type "Float (double-precision)") (TriggeredSeconds :type "Float (double-precision)") (InputAction :type "InputAction Object Reference" :default "/Game/Original/Input/InputAsset/Rotation.Rotation"))
  (bind (_x _y) (`KismetMathLibrary.BreakVector2D` ActionValue))
  (bind _arrow (`self.Arrow`))
  (bind (_relativerotation_roll _relativerotation_pitch _relativerotation_yaw) (`KismetMathLibrary.BreakRotator` (`SceneComponent.RelativeRotation` _arrow)))
  (:`Triggered`
    (`SceneComponent.K2_SetRelativeRotation` _arrow (`KismetMathLibrary.MakeRotator` _relativerotation_roll (`KismetMathLibrary.FClamp` (+ _relativerotation_pitch _y) -25.0 25.0) (+ _relativerotation_yaw _x)) false false)
    (`KismetSystemLibrary.PrintString` "Hello")))

(event `EnhancedInput|/Game/Original/Input/InputAsset/Distance`
  (params (ActionValue :type "Float (double-precision)") (ElapsedSeconds :type "Float (double-precision)") (TriggeredSeconds :type "Float (double-precision)") (InputAction :type "InputAction Object Reference" :default "/Game/Original/Input/InputAsset/Distance.Distance"))
  (bind _springarm (`self.SpringArm`))
  (:`Triggered`
    (set `SpringArmComponent.TargetArmLength` (`KismetMathLibrary.FClamp` (+ (* ActionValue 100.0) (`SpringArmComponent.TargetArmLength` _springarm)) 300.0 500.0) _springarm)))

(fn `UserConstructionScript`)